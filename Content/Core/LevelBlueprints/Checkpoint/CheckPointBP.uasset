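; CheckPointBP is a checkpoint trigger that saves a respawn transform when a WallWalker overlaps its collision box.
; It loads the existing CheckPointSaveGame from its slot or creates a new one, then writes the checkpoint's transform, raised slightly with unit scale, and saves it.
; The construction script sizes the box from X, Y and Z variables.
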(event OnComponentBeginOverlap(CheckPointCollision)
  (params (OverlappedComponent :type Primitive%20Component%20Object%20Reference) (OtherActor :type Actor%20Object%20Reference) (OtherComp :type Primitive%20Component%20Object%20Reference) (OtherBodyIndex :type Integer) (bFromSweep :type Boolean) (SweepResult :type Hit%20Result%20Structure%20%28by%20ref%29))
  (bind _returnvalue (Transformation|GetActorTransform))
  (Utilities|Casting|CastToWallWalker OtherActor)
  (bind _returnvalue_2 (SaveGame|DoesSaveGameExist (Variables|Default|GetCheckpointSaveName)))
  (if _returnvalue_2
    (bind _returnvalue_3 (SaveGame|LoadGamefromSlot (Variables|Default|GetCheckpointSaveName)))
    (bind _ascheck_point_save_game (Utilities|Casting|CastToCheckPointSaveGame _returnvalue_3))
    (Variables|Default|SetSaveGameRef _ascheck_point_save_game)
    (else
      (bind _returnvalue_4 (SaveGame|CreateSaveGameObject "/Game/Core/LevelBlueprints/Checkpoint/CheckPointSaveGame.CheckPointSaveGame_C"))
      (Variables|Default|SetSaveGameRef _returnvalue_4)))
  (bind _output_get (Variables|/Game/Core/LevelBlueprints/Checkpoint/CheckPointSaveGame.CheckPointSaveGame_C|SetCheckpoint (Variables|Default|GetSaveGameRef) (Math|Transform|MakeTransform (+ (.location _returnvalue) "0, 0,100.000000") (.rotation _returnvalue))))
  (SaveGame|SaveGametoSlot (Variables|Default|GetSaveGameRef) (Variables|Default|GetCheckpointSaveName)))

(fn ConstructionScript
  (Components|Box|SetBoxExtent (Variables|Default|GetCheckPointCollision) (Math|Vector|MakeVector (Variables|Default|GetX) (Variables|Default|GetY) (Variables|Default|GetZ)) true))